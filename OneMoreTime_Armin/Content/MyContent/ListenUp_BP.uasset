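; ListenUp_BP is a sound-emitting shooting target that times how quickly the player hits it.
; Each reset shows the cube, places it at a fixed distance within a random yaw range relative to the player's facing, plays audio and starts the timer.
; ShootEvent prints the reaction time, hides the cube and disables its collision, then respawns it after a delay.
; Debug lines mark the spawn arc's bounds.
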(event Custom|ResetTarget
  (bind _cube (Variables|Default|GetCube))
  (Rendering|SetVisibility _cube true false)
  (Collision|SetCollisionEnabled _cube "QueryOnly")
  (Transformation|SetActorLocation (+ (Math|Vector|RotateVector (Math|Vector|MakeVector 0.0 (Variables|Default|GetSpawnDistance) 0.0) (Math|Rotator|MakeRotator 0.0 0.0 (+ (Utilities|GetPlayerForwardZValue) (Math|Random|RandomFloatinRange (Variables|Default|GetRightBound) (Variables|Default|GetLeftBound))))) (Transformation|GetActorLocation (Pawn|GetControlledPawn (Game|GetPlayerController 0)))) false false)
  (Audio|Components|Audio|Play (Variables|Default|GetAudio) 0.0)
  (Variables|Default|SetReactionTimeReference (Utilities|Time|GetTimeSeconds)))

(event Custom|DrawBounds
  (bind _returnvalue (Game|GetPlayerController 0))
  (bind _returnvalue_2 (Pawn|GetControlledPawn _returnvalue))
  (bind _returnvalue_3 (Transformation|GetActorLocation _returnvalue_2))
  (Rendering|Debug|DrawDebugLine :LineStart _returnvalue_3 :LineEnd (+ (Math|Vector|RotateVector (Math|Vector|MakeVector 0.0 (Variables|Default|GetSpawnDistance) 0.0) (Math|Rotator|MakeRotator 0.0 0.0 (+ (Utilities|GetPlayerForwardZValue) (Variables|Default|GetRightBound)))) _returnvalue_3) :Duration 1e+02 :Thickness 4.0)
  (Rendering|Debug|DrawDebugLine :LineStart _returnvalue_3 :LineEnd (+ (Math|Vector|RotateVector (Math|Vector|MakeVector 0.0 (Variables|Default|GetSpawnDistance) 0.0) (Math|Rotator|MakeRotator 0.0 0.0 (+ (Utilities|GetPlayerForwardZValue) (Variables|Default|GetLeftBound)))) _returnvalue_3) :Duration 1e+02 :Thickness 4.0))

(event EventBeginPlay
  (CallFunction|DrawBounds)
  (CallFunction|ResetTarget))

(event EventShootEvent
  (bind _cube (Variables|Default|GetCube))
  (Development|PrintString "Listen Hit")
  (Development|PrintString (Utilities|String|ToString(Float) (- (Utilities|Time|GetTimeSeconds) (Variables|Default|GetReactionTimeReference))))
  (Rendering|SetVisibility _cube false false)
  (Collision|SetCollisionEnabled _cube "NoCollision")
  (Utilities|FlowControl|Delay (Variables|Default|GetTargetRespawnTime))
  (CallFunction|ResetTarget)
  (CallFunction|DrawBounds))

(fn ConstructionScript)