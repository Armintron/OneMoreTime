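; Memorabilia actor that builds a vertical grid of child actors at BeginPlay and makes each one wiggle.
; It briefly spawns ActorToSpawn out of the way to measure its X bounds, deriving cell spacing plus percentage padding.
; Child actor components fill the rows and columns in the XZ plane, then each TestBP child receives Wiggle with shared settings.
; ShootEvent is an empty stub.
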(event EventBeginPlay
  (bind _returnvalue (Game|SpawnActorfromClass (Variables|Default|GetActorToSpawn) (Math|Transform|MakeTransform "-1000.000000,-1000.000000,-1000.000000" "0, 0, 0" "1,1,1") "Undefined" 0 0))
  (Variables|GridParameters|SetGridSpacing (+ (* (.x (.BoxExtent (Collision|GetActorBounds _returnvalue false))) 2.0) (* (* (.x (.BoxExtent (Collision|GetActorBounds _returnvalue false))) 2.0) (* (Variables|GridParameters|GetGridPadding%20%28%25%29) 0.01))))
  (Actor|DestroyActor _returnvalue)
  (for _index (range 1 (Variables|GridParameters|GetGridHeight%20%28Rows%29))
    (for _index_2 (range 1 (Variables|GridParameters|GetGridWidth%20%28Columns%29))
      (bind _returnvalue_2 (AddComponent|AddChildActorComponent false (Math|Transform|MakeTransform (Math|Vector|MakeVector (* _index_2 (Variables|GridParameters|GetGridSpacing)) 0.0 (* _index (Variables|GridParameters|GetGridSpacing))))))
      (Utilities|Array|Add (Variables|Default|GetModelList) _returnvalue_2)))
  (for _array_element (Variables|Default|GetModelList)
    (Default|Wiggle (.AsTest%20BP (Utilities|Casting|CastToTestBP (Variables|/Script/Engine.ChildActorComponent|GetChildActor _array_element))) (Variables|WiggleParameters|GetWiggleSpeed%20%28Multiplier%29) (Variables|WiggleParameters|GetWiggleDuration) (Variables|WiggleParameters|GetWiggleAmount))))

(event EventShootEvent)

(fn ConstructionScript)