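; ToddlerTime_Item_BP is a physics item that can be picked up and dropped by BP_MotionController.
; On BeginPlay it picks a random ItemNumber from 0 to 2, which nothing else in this graph uses.
; Pickup disables mesh physics and attaches the root to the given component at its world transform, while Drop re-enables physics and detaches the actor.
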(event EventBeginPlay
  (Variables|Default|SetItemNumber (Math|Random|RandomIntegerinRange 0 2)))

(event EventPickup
  (params (AttachTo :type Scene%20Component%20Object%20Reference))
  (Physics|SetSimulatePhysics (Variables|Default|GetStaticMeshComponent) false)
  (Transformation|AttachComponentToComponent (VehicleSound|GetRootComponent) AttachTo "None" "KeepWorld" "KeepWorld" "KeepWorld" false))

(event EventDrop
  (Physics|SetSimulatePhysics (Variables|Default|GetStaticMeshComponent) true)
  (Transformation|DetachFromActor "KeepWorld" "KeepWorld" "KeepWorld"))

(fn ConstructionScript
  (|CallParentFunction))