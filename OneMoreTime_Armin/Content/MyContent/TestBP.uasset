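; Shootable actor for what looks like a guessing game, randomly marked correct at BeginPlay, which also makes its static mesh visible.
; Wiggle jitters it with random offsets at a given rate, stops timeline looping after a timed delay, then eases it back to relative origin and flips it 180 degrees.
; ShootEvent fires once, calling Reveal to reverse the flip timeline and playing a click sound if correct.
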(event Custom|Wiggle
  (params (WiggleRate%20%28Multiplier%29 :type Float%20%28single-precision%29%20%28by%20ref%29) (WiggleDuration :type Integer%20%28by%20ref%29) (WiggleAmount :type Float%20%28single-precision%29%20%28by%20ref%29))
  (bind _returnvalue (Math|Random|RandomFloatinRange 0.0 WiggleAmount))
  (bind _wiggletimeline (Variables|Default|GetWiggleTimeline))
  (bind _returnvalue_2 (* -1 _returnvalue))
  (Utilities|FlowControl|Sequence
    (:then_0
      (Components|Timeline|SetPlayRate (Variables|Default|GetWiggleTimeline) WiggleRate%20%28Multiplier%29)
      (bind _wiggletrack (Timeline|WiggleTimeline Play)
        (:Update
          (Transformation|AddActorLocalOffset (Math|Vector|Lerp(Vector) (Math|Vector|MakeVector _returnvalue_2 0.0 _returnvalue_2) (Math|Vector|MakeVector _returnvalue 0.0 _returnvalue) _wiggletrack) false false))
        (:Finished
          ;[1 1 1] Reset Position
          (bind _testingalpha (Timeline|WiggleRest Play)
            (:Update
              (Transformation|SetActorRelativeLocation (Math|Vector|Lerp(Vector) (.location (Transformation|GetRelativeTransform (Variables|Default|GetDefaultSceneRoot))) "0, 0, 0" _testingalpha)))
            (:Finished
              (bind _testingalpha_2 (Timeline|Flip180 Play)
                (:Update
                  (Transformation|SetActorRelativeRotation (Math|Rotator|Lerp(Rotator) "0, 0, 0" "0.000000,180.000000, 0" _testingalpha_2)))))))))
    (:then_1
      (Utilities|FlowControl|Delay (* WiggleDuration (Components|Timeline|GetTimelineLength _wiggletimeline)))
      (Components|Timeline|SetLooping _wiggletimeline false))))

(event Custom|Reveal
  ;[1 1 1] Reset Position
  (bind _testingalpha (Timeline|Flip180 ReverseFromEnd)
    (:Update
      (Transformation|SetActorRelativeRotation (Math|Rotator|Lerp(Rotator) "0, 0, 0" "0.000000,180.000000, 0" _testingalpha)))))

(event EventShootEvent
  (Utilities|FlowControl|DoOnce false
    (:Completed
      (CallFunction|Reveal)
      (if (Variables|Default|GetCorrect?)
        (Audio|PlaySound2D "/Engine/VREditor/Sounds/UI/Click_on_Button.Click_on_Button" 1.0 1.0 0.0 0 0)))))

(event EventBeginPlay
  (if (Math|Random|RandomBool)
    (Rendering|SetVisibility (Variables|Default|GetStaticMesh) true false)
    (Variables|Default|SetCorrect? true)))

(fn ConstructionScript)